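; BP_BreakableBlock is a breakable crate that drops a random item when destroyed.
; Its Geometry Collection's Chaos break event plays an explosion sound and spawns a cone, cube, cylinder or capsule item at the actor's location, each equally likely.
; The spawned item receives a reference to the crate through SetCrate.
; A HasSpawned flag, reset on BeginPlay, limits the sound and drop to the first break event.
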(event OnChaosBreakEvent(GeometryCollectionComponent)
  (params (BreakEvent :type Chaos%20Break%20Event%20Structure%20%28by%20ref%29))
  (bind _returnvalue (Transformation|GetActorLocation))
  (bind _returnvalue_2 (Transformation|GetActorLocation))
  (bind _returnvalue_3 (Math|Conversions|ToTransform(Vector) _returnvalue))
  (bind _returnvalue_4 (Math|Conversions|ToTransform(Vector) _returnvalue_2))
  (if (not (Variables|Default|GethasSpawned))
    (Audio|PlaySoundatLocation "/Game/Sound/medium-explosion-40472.medium-explosion-40472" (Transformation|GetWorldLocation (Variables|Default|GetGeometryCollectionComponent)) "0, 0, 0" 1.0 1.0 0.0 0 0 0 0)
    (Variables|Default|SethasSpawned true)
    (switch int (Math|Random|RandomInteger 4)
      (:0
        (bind _returnvalue_5 (Game|SpawnActorfromClass "/Game/LevelItems/BP_ConeItem.BP_ConeItem_C" _returnvalue_4 "Undefined" 0 0))
        (Utilities|IsValid _returnvalue_5
          (:Is%20Valid
            (Class|UnrealChallenge2Item|SetCrate _returnvalue_5 self))))
      (:1
        (bind _returnvalue_6 (Game|SpawnActorfromClass "/Game/LevelItems/BP_CubeItem.BP_CubeItem_C" _returnvalue_4 "Undefined" 0 0))
        (Utilities|IsValid _returnvalue_6
          (:Is%20Valid
            (Class|UnrealChallenge2Item|SetCrate _returnvalue_6 self))))
      (:2
        (bind _returnvalue_7 (Game|SpawnActorfromClass "/Game/LevelItems/BP_CylinderItem.BP_CylinderItem_C" _returnvalue_3 "Undefined" 0 0))
        (Utilities|IsValid _returnvalue_7
          (:Is%20Valid
            (Class|UnrealChallenge2Item|SetCrate _returnvalue_7 self))))
      (:3
        (bind _returnvalue_8 (Game|SpawnActorfromClass "/Game/LevelItems/BP_CapsuleItem.BP_CapsuleItem_C" _returnvalue_3 "Undefined" 0 0))
        (Utilities|IsValid _returnvalue_8
          (:Is%20Valid
            (Class|UnrealChallenge2Item|SetCrate _returnvalue_8 self)))))))

(event EventBeginPlay
  (Variables|Default|SethasSpawned false))

(fn ConstructionScript)